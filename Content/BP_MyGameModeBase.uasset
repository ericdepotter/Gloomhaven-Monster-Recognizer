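; Game mode Blueprint that builds lookup tables of monster textures and masks from the project's content folders.
; Its LoadMonsterTexturesandMasks event queries the Asset Registry for both folders and stores each Texture2D in MonsterTextures or MonsterMasks, keyed by asset name.
; Mask keys have "_mask" removed to match texture names, and both passes also add their names to MonsterNames.
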(event EventLoadMonsterTexturesandMasks
  (bind _returnvalue (Class|AssetRegistryHelpers|GetAssetRegistry))
  (Utilities|FlowControl|Sequence
    (:then_0
      (bind _outassetdata (Class|AssetRegistry|GetAssetsbyPath _returnvalue "/Game/Monsters/Textures" false false))
      (for _array_element _outassetdata
        (bind _astexture_2d (Utilities|Casting|CastToTexture2D (Class|AssetRegistryHelpers|GetAsset _array_element)))
        (Utilities|Map|Add (Variables|Default|GetMonsterTextures) (Utilities|String|ToString(Name) (.AssetName (Utilities|Struct|BreakAssetData _array_element))) _astexture_2d)
        (Utilities|Set|Add (Variables|Default|GetMonsterNames) (Utilities|String|ToString(Name) (.AssetName (Utilities|Struct|BreakAssetData _array_element))))))
    (:then_1
      (bind _outassetdata_2 (Class|AssetRegistry|GetAssetsbyPath _returnvalue "/Game/Monsters/Masks" false false))
      (for _array_element_2 _outassetdata_2
        (bind _astexture_2d_2 (Utilities|Casting|CastToTexture2D (Class|AssetRegistryHelpers|GetAsset _array_element_2)))
        (Utilities|Map|Add (Variables|Default|GetMonsterMasks) (Utilities|String|Replace (Utilities|String|ToString(Name) (.AssetName (Utilities|Struct|BreakAssetData _array_element_2))) "_mask") _astexture_2d_2)
        (Utilities|Set|Add (Variables|Default|GetMonsterNames) (Utilities|String|Replace (Utilities|String|ToString(Name) (.AssetName (Utilities|Struct|BreakAssetData _array_element_2))) "_mask"))))))

(fn ConstructionScript)