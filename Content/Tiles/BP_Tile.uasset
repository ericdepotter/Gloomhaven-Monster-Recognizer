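; BP_Tile is a tile actor that spawns monsters and keeps track of them.
; On BeginPlay it hides all its SpawnLocation components, caching the static mesh's first material as TileMaterial inside the same loop.
; Its SpawnMonster event spawns a BP_Monster at a supplied location and rotation and adds it to the Monsters array.
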(event EventBeginPlay
  (for _array_element (Actor|GetComponentsByClass self "/Script/GloomhavenReco.SpawnLocation")
    (Rendering|SetVisibility _array_element false false)
    (Variables|Default|SetTileMaterial (Rendering|Material|GetMaterial (Variables|Default|GetStaticMeshComponent) 0))))

(event EventSpawnMonster
  (params (Location :type Vector :default "0, 0, 0") (Rotation :type Rotator :default "0, 0, 0"))
  (bind _returnvalue (Game|SpawnActorfromClass "/Game/Monsters/BP_Monster.BP_Monster_C" (Math|Transform|MakeTransform Location Rotation) "Undefined" 0 0))
  (Utilities|Array|Add (Variables|Default|GetMonsters) _returnvalue))

(fn ConstructionScript)