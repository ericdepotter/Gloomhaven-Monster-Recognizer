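; BP_Monster is a monster actor shown on a Plane, which can display either the monster's texture or its mask.
; On BeginPlay it nudges the plane by a small random X/Y offset and yaw, so placement varies slightly.
; SwitchtoTexture and SwitchtoMask each fetch an image from the GameMode by MonsterName and apply it through a newly created M_Monster dynamic material instance.
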(event EventBeginPlay
  (Utilities|FlowControl|Sequence
    (:then_0
      (Transformation|AddLocalOffset (Variables|Default|GetPlane) (Math|Vector|MakeVector (Math|Random|RandomFloatinRange -1.5 1.5) (Math|Random|RandomFloatinRange -0.4 0.7) 0.0) false false)
      (Transformation|AddLocalRotation (Variables|Default|GetPlane) (Math|Rotator|MakeRotator 0.0 0.0 (Math|Random|RandomFloatinRange -3.0 3.0)) false false))))

(event EventSwitchtoTexture
  (bind _returnvalue (Rendering|Material|CreateDynamicMaterialInstance "/Game/Monsters/M_Monster.M_Monster" "None" :!class /Script/Engine.KismetMaterialLibrary))
  (Rendering|Material|SetMaterial (Variables|Default|GetPlane) 0 _returnvalue)
  (Rendering|Material|SetTextureParameterValue _returnvalue "MonsterTexture" (Class|MyGameModeBase|GetMonsterTexture (Variables|Default|GetGameMode) (Variables|Default|GetMonsterName))))

(event EventSwitchtoMask
  (bind _returnvalue (Rendering|Material|CreateDynamicMaterialInstance "/Game/Monsters/M_Monster.M_Monster" "None" :!class /Script/Engine.KismetMaterialLibrary))
  (Rendering|Material|SetMaterial (Variables|Default|GetPlane) 0 _returnvalue)
  (Rendering|Material|SetTextureParameterValue _returnvalue "MonsterTexture" (Class|MyGameModeBase|GetMonsterMask (Variables|Default|GetGameMode) (Variables|Default|GetMonsterName))))

(fn ConstructionScript)