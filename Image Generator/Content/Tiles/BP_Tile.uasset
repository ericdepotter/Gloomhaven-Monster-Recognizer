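; BP_Tile is a tile actor that carries spawn location markers and can spawn monsters.
; On BeginPlay it counts its SpawnLocation components, hides each one and caches the tile mesh's first material inside that same loop.
; Its SpawnMonster event creates a BP_Monster at the supplied location and rotation, then appends it to the tile's Monsters array.
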(event EventBeginPlay
  (bind _self self)
  (bind _returnvalue (Actor|GetComponentsByClass _self "/Script/GloomhavenReco.SpawnLocation"))
  (Variables|Default|SetNumberSpawnPoints (Utilities|Array|Length _returnvalue))
  (for _array_element _returnvalue
    (Rendering|SetVisibility _array_element false false)
    (Variables|Default|SetTileMaterial (Rendering|Material|GetMaterial (Variables|Default|GetStaticMeshComponent) 0))))

(event EventSpawnMonster
  (params (Location :type Vector :default "0, 0, 0") (Rotation :type Rotator :default "0, 0, 0"))
  (bind _returnvalue (Game|SpawnActorfromClass "/Game/Monsters/BP_Monster.BP_Monster_C" (Math|Transform|MakeTransform Location Rotation) "Undefined" 0 0))
  (Utilities|Array|Add (Variables|Default|GetMonsters) _returnvalue))

(fn ConstructionScript)