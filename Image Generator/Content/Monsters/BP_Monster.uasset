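; BP_Monster is a monster standee actor that randomizes its look on spawn and can switch between textured, mask and black display states.
; BeginPlay jitters the monster mesh's offset and yaw, rolls a 25% elite chance and creates dynamic materials for monster and standee.
; Switch events drive material parameters using textures or masks fetched by MonsterName from the GameMode.
; The standee shows elite status only in the textured state and turns black otherwise.
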(event EventBeginPlay
  (Utilities|FlowControl|Sequence
    (:then_0
      (Transformation|AddLocalOffset (Variables|Default|GetMonster) (Math|Vector|MakeVector (Math|Random|RandomFloatinRange -1.5 1.5) (Math|Random|RandomFloatinRange -0.4 0.7) 0.0) false false)
      (Transformation|AddLocalRotation (Variables|Default|GetMonster) (Math|Rotator|MakeRotator 0.0 0.0 (Math|Random|RandomFloatinRange -3.0 3.0)) false false))
    (:then_1
      (Variables|Default|SetbIsElite (< (Math|Random|RandomFloatinRange 0.0 1.0) 0.25)))
    (:then_2
      (bind _returnvalue (Rendering|Material|CreateDynamicMaterialInstance "/Game/Monsters/M_Monster.M_Monster" "None" :!class /Script/Engine.KismetMaterialLibrary))
      (Rendering|Material|SetMaterial (Variables|Default|GetMonster) 0 _returnvalue))
    (:then_3
      (bind _returnvalue_2 (Rendering|Material|CreateDynamicMaterialInstance "/Game/Monsters/M_MonsterStandee.M_MonsterStandee" "None" :!class /Script/Engine.KismetMaterialLibrary))
      (Rendering|Material|SetMaterial (Variables|Default|GetStandee) 0 _returnvalue_2))))

(event EventSwitchtoBlack
  (Rendering|Material|SetScalarParameterValue (stale EventBeginPlay _returnvalue) "bIsBlack" 1.0 :!class /Script/Engine.MaterialInstanceDynamic)
  (Rendering|Material|SetMaterial (Variables|Default|GetStandee) 0 "/Game/M_Black.M_Black"))

(event EventSwitchtoTexture
  (Rendering|Material|SetTextureParameterValue (stale EventBeginPlay _returnvalue) "MonsterTexture" (Class|MyGameModeBase|GetMonsterTexture (Variables|Default|GetGameMode) (Variables|Default|GetMonsterName)))
  (Rendering|Material|SetScalarParameterValue (stale EventBeginPlay _returnvalue) "bIsMask" 0.0 :!class /Script/Engine.MaterialInstanceDynamic)
  (Rendering|Material|SetScalarParameterValue (stale EventBeginPlay _returnvalue) "bIsBlack" 0.0 :!class /Script/Engine.MaterialInstanceDynamic)
  (Rendering|Material|SetScalarParameterValue (stale EventBeginPlay _returnvalue_2) "bIsElite" (Math|Conversions|ToFloat(Boolean) (Variables|Default|GetbIsElite)) :!class /Script/Engine.MaterialInstanceDynamic)
  (Rendering|Material|SetMaterial (Variables|Default|GetStandee) 0 (stale EventBeginPlay _returnvalue_2)))

(event EventSwitchtoMask
  (Rendering|Material|SetTextureParameterValue (stale EventBeginPlay _returnvalue) "MonsterTexture" (Class|MyGameModeBase|GetMonsterMask (Variables|Default|GetGameMode) (Variables|Default|GetMonsterName)))
  (Rendering|Material|SetScalarParameterValue (stale EventBeginPlay _returnvalue) "bIsMask" 1.0 :!class /Script/Engine.MaterialInstanceDynamic)
  (Rendering|Material|SetScalarParameterValue (stale EventBeginPlay _returnvalue) "bIsBlack" 0.0 :!class /Script/Engine.MaterialInstanceDynamic)
  (Rendering|Material|SetMaterial (Variables|Default|GetStandee) 0 "/Game/M_Black.M_Black"))

(fn ConstructionScript)